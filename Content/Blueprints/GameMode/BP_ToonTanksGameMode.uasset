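; BP_ToonTanksGameMode is the Toon Tanks game mode Blueprint that puts the match UI on screen.
; On StartGame it creates the start-game widget and the player health widget and adds both to the viewport.
; On GameOver it shows the end-game widget and sets its text to a win or game-over message based on the WonGame flag.
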(event `self.StartGame`
  (`|ExecutionSequence`
    (:`then_0`
      (bind _returnvalue (`|CreateWidget` "/Game/Blueprints/Widgets/WBP_StartGameWidget.WBP_StartGameWidget_C"))
      (`UserWidget.AddToViewport` _returnvalue 0))
    (:`then_1`
      (bind _returnvalue_2 (`|CreateWidget` "/Game/Blueprints/Widgets/WBP_PlayerHealth.WBP_PlayerHealth_C"))
      (`UserWidget.AddToViewport` _returnvalue_2 0))))

(event `self.GameOver`
  (params (bWonGame :type Boolean))
  (bind _returnvalue (`|CreateWidget` "/Game/Blueprints/Widgets/WBP_EndGameWidget.WBP_EndGameWidget_C"))
  (`UserWidget.AddToViewport` _returnvalue 0)
  (`TextBlock.SetText` (`/Game/Blueprints/Widgets/WBP_EndGameWidget.DisplayText` _returnvalue) (select `bool` bWonGame :`false` "GAME OVER" :`true` "YOU WON!!" :!type "Text")))

(fn `UserConstructionScript`)